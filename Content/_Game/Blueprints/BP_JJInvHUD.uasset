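; HUD Blueprint that draws the player's crosshair texture on screen.
; Each DrawHUD, it reads CrosshairOffset from the JJInvCharacter player pawn and recomputes the screen center from the current viewport size.
; It draws the fixed-size crosshair at center plus that offset, shifted by HalfWidth and HalfHeight, so the character controls where the reticle sits.
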(event EventDrawHUD
  (params (SizeX :type Integer) (SizeY :type Integer))
  (bind _screencenter (Variables|Default|GetScreenCenter))
  (bind _asjjinv_character (Utilities|Casting|CastToJJInvCharacter (Game|GetPlayerCharacter 0)))
  (Variables|Default|SetBPCrosshairOffset (Variables|/Script/JJInv.JJInvCharacter|GetCrosshairOffset _asjjinv_character))
  (CallFunction|SetScreenCenter SizeX SizeY)
  (Canvas|DrawTexture "/Game/_Game/Assets/Textures/Crosshairs/Cross_Q_9.Cross_Q_9" (- (+ (.x _screencenter) (.x (Variables|Default|GetBPCrosshairOffset))) (Variables|Default|GetHalfWidth)) (- (+ (.y _screencenter) (.y (Variables|Default|GetBPCrosshairOffset))) (Variables|Default|GetHalfHeight)) 64.0 64.0 0.0 0.0 1.0 1.0 "(R=1.000000,G=1.000000,B=1.000000,A=1.000000)"))

(fn ConstructionScript)

(fn SetScreenCenter
  (params (A :type Integer) (A2 :type Integer))
  (Variables|Default|SetScreenCenter (Math|Vector2D|MakeVector2D (Math|Conversions|ToFloat(Integer) (/ A 2)) (Math|Conversions|ToFloat(Integer) (/ A2 2)))))